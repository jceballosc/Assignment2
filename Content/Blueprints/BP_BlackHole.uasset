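; BP_BlackHole is a black hole actor that pulls every BP_Ship toward its Horizont component.
; Each tick it finds all ships and adds a fixed-size velocity toward Horizont to each Player component, independent of distance and not scaled by delta time.
; An unconnected branch would instead set the velocity of BP_Debug cubes toward the same point.
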(event EventTick
  (params (DeltaSeconds :type Float%20%28single-precision%29))
  (bind _outactors (Actor|GetAllActorsOfClass "/Game/Blueprints/BP_Ship.BP_Ship_C"))
  (for _array_element _outactors
    (Class|PrimitiveComponent|SetAllPhysicsLinearVelocity (Variables|/Game/Blueprints/BP_Ship.BP_Ship_C|GetPlayer _array_element) (* (Math|Vector|GetForwardVector (Math|Rotator|FindLookatRotation (Transformation|GetWorldLocation (Variables|/Game/Blueprints/BP_Ship.BP_Ship_C|GetPlayer _array_element)) (Transformation|GetWorldLocation (Variables|Default|GetHorizont)))) 2.0) true)))

(fn ConstructionScript)