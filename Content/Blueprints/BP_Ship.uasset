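; BP_Ship is a ship Blueprint that switches its bottom, left and right thruster components on and off.
; Two events, ActivateThrust and DeactivateThrust, take a thruster ID and select the matching component.
; Each checks the component's active state first, so it only activates or deactivates on an actual change, without resetting a running thruster.
; It contains no input or movement logic, and the construction script is empty.
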(event Custom|ActivateThrust
  (params (ThrusterID :type Integer))
  (switch int ThrusterID
    (:0
      (if (not (Components|Activation|IsActive (Variables|Default|GetBottomThruster)))
        (Components|Activation|Activate (Variables|Default|GetBottomThruster) false)))
    (:1
      (if (not (Components|Activation|IsActive (Variables|Default|GetLeftThruster)))
        (Components|Activation|Activate (Variables|Default|GetLeftThruster) false)))
    (:2
      (if (not (Components|Activation|IsActive (Variables|Default|GetRightThruster)))
        (Components|Activation|Activate (Variables|Default|GetRightThruster) false)))))

(event Custom|DeactivateThrust
  (params (ThrusterID :type Integer))
  (switch int ThrusterID
    (:0
      (if (Components|Activation|IsActive (Variables|Default|GetBottomThruster))
        (Components|Activation|Deactivate (Variables|Default|GetBottomThruster))))
    (:1
      (if (Components|Activation|IsActive (Variables|Default|GetLeftThruster))
        (Components|Activation|Deactivate (Variables|Default|GetLeftThruster))))
    (:2
      (if (Components|Activation|IsActive (Variables|Default|GetRightThruster))
        (Components|Activation|Deactivate (Variables|Default|GetRightThruster))))))

(fn ConstructionScript)