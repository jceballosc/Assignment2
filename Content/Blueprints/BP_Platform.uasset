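; BP_Platform is a platform actor that detects a player within its Collider and destroys players that hit it too fast.
; Unless it is the starting platform, overlap by a BPI_Player actor starts a looping timer, cleared on exit.
; The timer compares bounds to check full containment along Y, currently only printing a debug message.
; Platform hits destroy the player when its velocity reaches a threshold, including on the starting platform.
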(event OnComponentBeginOverlap(Collider)
  (params (OverlappedComponent :type Primitive%20Component%20Object%20Reference) (OtherActor :type Actor%20Object%20Reference) (OtherComp :type Primitive%20Component%20Object%20Reference) (OtherBodyIndex :type Integer) (bFromSweep :type Boolean) (SweepResult :type Hit%20Result%20Structure%20%28by%20ref%29))
  (if (and (Utilities|DoesObjectImplementInterface OtherActor "/Game/Framework/BPI_Player.BPI_Player_C") (not (Variables|Default|GetisStartingPlatform)))
    (Variables|Default|SetOverlappedActor OtherActor)
    (bind _returnvalue (Utilities|Time|SetTimerbyFunctionName 0 "isPlayerInCollider" 0.1 true))
    (Variables|Default|SetCollisionTimer _returnvalue)))

(event OnComponentEndOverlap(Collider)
  (params (OverlappedComponent :type Primitive%20Component%20Object%20Reference) (OtherActor :type Actor%20Object%20Reference) (OtherComp :type Primitive%20Component%20Object%20Reference) (OtherBodyIndex :type Integer))
  (if (and (Utilities|DoesObjectImplementInterface OtherActor "/Game/Framework/BPI_Player.BPI_Player_C") (not (Variables|Default|GetisStartingPlatform)))
    (Utilities|Time|ClearandInvalidateTimerbyHandle (Variables|Default|GetCollisionTimer))))

(event OnComponentHit(Platform)
  (params (HitComponent :type Primitive%20Component%20Object%20Reference) (OtherActor :type Actor%20Object%20Reference) (OtherComp :type Primitive%20Component%20Object%20Reference) (NormalImpulse :type Vector :default "0, 0, 0") (Hit :type Hit%20Result%20Structure%20%28by%20ref%29))
  (if (and (Utilities|DoesObjectImplementInterface OtherActor "/Game/Framework/BPI_Player.BPI_Player_C") (>= (Math|Vector|VectorLength (Transformation|GetVelocity OtherActor)) 6e+01))
    (Actor|DestroyActor OtherActor)))

(event Custom|isPlayerInCollider
  (bind _collider (Variables|Default|GetCollider))
  (bind _overlappedactor (Variables|Default|GetOverlappedActor))
  (bind (_origin _boxextent) (Collision|GetComponentBounds _collider))
  (bind (_origin_2 _boxextent_2) (Collision|GetActorBounds _overlappedactor false false))
  (if (<= (Math|Float|Absolute(Float) (- (.y _origin) (.y _origin_2))) (- (.y _boxextent) (.y _boxextent_2)))
    (Development|PrintString "INBOUNDS")))

(fn ConstructionScript)