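; Player controller for a lander game that routes input to the BP_Ship in the level.
; It caches the first BP_Ship found at BeginPlay, then maps bottom, left and right thruster actions to indexed ActivateThrust and DeactivateThrust calls.
; Up and Right axes apply vertical (scaled up) and Y-axis force to the ship's Player outside a small dead zone.
; Only bottom thruster and Up handlers check validity.
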(event EventBeginPlay
  (bind _outactors (Actor|GetAllActorsOfClass "/Game/Blueprints/BP_Ship.BP_Ship_C"))
  (Variables|Default|SetShip (Utilities|Array|Get(acopy) _outactors)))

(event Input|ActionEvents|InputActionBottomThruster
  (params (Key :type Key%20Structure :default "None"))
  (bind _ship (Variables|Default|GetShip))
  (:Pressed
    (Utilities|IsValid _ship
      (:Is%20Valid
        (Default|ActivateThrust _ship))))
  (:Released
    (Utilities|IsValid _ship
      (:Is%20Valid
        (Default|DeactivateThrust _ship)))))

(event Input|ActionEvents|InputActionLeftThruster
  (params (Key :type Key%20Structure :default "None"))
  (:Pressed
    (Default|ActivateThrust (Variables|Default|GetShip) 1))
  (:Released
    (Default|DeactivateThrust (Variables|Default|GetShip) 1)))

(event Input|ActionEvents|InputActionRightThruster
  (params (Key :type Key%20Structure :default "None"))
  (:Pressed
    (Default|ActivateThrust (Variables|Default|GetShip) 2))
  (:Released
    (Default|DeactivateThrust (Variables|Default|GetShip) 2)))

(event Input|AxisEvents|InputAxisUp
  (params (AxisValue :type Float%20%28single-precision%29))
  (bind _ship (Variables|Default|GetShip))
  (bind _player (Variables|/Game/Blueprints/BP_Ship.BP_Ship_C|GetPlayer _ship))
  (if (not (Math|Float|NearlyEqual(Float) AxisValue 0.0 0.01))
    (Utilities|IsValid _player
      (:Is%20Valid
        (Physics|AddForce _player (Math|Vector|MakeVector 0.0 0.0 (* AxisValue 5.0)) "None" false)))))

(event Input|AxisEvents|InputAxisRight
  (params (AxisValue :type Float%20%28single-precision%29))
  (if (not (Math|Float|NearlyEqual(Float) AxisValue 0.0 0.01))
    (Physics|AddForce (Variables|/Game/Blueprints/BP_Ship.BP_Ship_C|GetPlayer (Variables|Default|GetShip)) (Math|Vector|MakeVector 0.0 AxisValue 0.0) "None" false)))

(fn ConstructionScript)